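; BP_Target is a target actor that switches its cube between target, missed and destroyed states, extending its parent class's handlers.
; The cube starts with physics-only collision and enables query collision only in the target state.
; Target and missed states swap materials, with missed returning to physics-only.
; Destruction disables queries, animates a DissolveAmount material parameter through a timeline, then calls the parent destroy logic when finished.
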(event EventDestroyTarget
  (Collision|SetCollisionEnabled (Variables|Default|GetCube) "PhysicsOnly")
  (bind _dissolvetrack (Timeline|DestroyTargetMaterial PlayFromStart)
    (:Update
      (Rendering|Material|SetScalarParameterValueonMaterials (Variables|Default|GetCube) "DissolveAmount" _dissolvetrack))
    (:Finished
      (|CallParentFunction))))

(event EventSetTargetState
  (|CallParentFunction)
  (Rendering|Material|SetMaterial (Variables|Default|GetCube) 0 "/Game/Materials/M_Target.M_Target")
  (Collision|SetCollisionEnabled (Variables|Default|GetCube) "QueryAndPhysics"))

(event EventSetMissedState
  (Rendering|Material|SetMaterial (Variables|Default|GetCube) 0 "/Game/Materials/M_TargetLost.M_TargetLost")
  (Collision|SetCollisionEnabled (Variables|Default|GetCube) "PhysicsOnly")
  (|CallParentFunction))

(event EventBeginPlay
  (Collision|SetCollisionEnabled (Variables|Default|GetCube) "PhysicsOnly"))

(fn ConstructionScript)